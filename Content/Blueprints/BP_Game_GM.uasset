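; Game mode for an asymmetric multiplayer game in which the first player to log in becomes the VR player and others play ghosts.
; It tracks player controllers and caches capture areas, player starts and the flashlight on BeginPlay.
; SpawnPlayer replaces a controller's pawn with a VR or third-person ghost pawn at a random start.
; Helpers count players within each capture area's radius for debug printing and move the flashlight to a supplied transform.
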(event EventBeginPlay
  (Utilities|FlowControl|Sequence
    (:then_0
      (bind _outactors (Actor|GetAllActorsOfClass "/Game/Blueprints/BP_CaptureArea.BP_CaptureArea_C"))
      (bind _output_get (Variables|Default|SetCaptureAreas _outactors))
      (Development|PrintString (Utilities|String|Append "Capture Areas: " (Utilities|String|ToString(Integer) (Utilities|Array|Length _output_get))) true true "(R=1.000000,G=0.097051,B=0.000000,A=1.000000)"))
    (:then_1
      (bind _outactors_2 (Actor|GetAllActorsOfClass "/Script/Engine.PlayerStart"))
      (bind _output_get_2 (Variables|Default|SetPlayerSpawns _outactors_2))
      (Development|PrintString (Utilities|String|Append "Player Starts: " (Utilities|String|ToString(Integer) (Utilities|Array|Length _output_get_2))) true true "(R=1.000000,G=0.097051,B=0.000000,A=1.000000)"))
    (:then_2
      (bind _returnvalue (Actor|GetActorOfClass "/Game/Blueprints/BP_Flashlight.BP_Flashlight_C"))
      (Variables|Default|SetFlashlight _returnvalue))))

(event EventPostLogin
  (params (NewPlayer :type Player%20Controller%20Object%20Reference))
  (bind _playercontrollers (Variables|Default|GetPlayerControllers))
  ;[0 0 0] Manage Connections
  ;;[1 1 1] On Player Login
  (bind _asbp_game_pc (Utilities|Casting|CastToBP_Game_PC NewPlayer))
  (Utilities|FlowControl|Sequence
    (:then_0
      (if (== (Utilities|Array|Length _playercontrollers) 0)
        (Variables|/Game/Blueprints/BP_Game_PC.BP_Game_PC_C|SetIsVR _asbp_game_pc true)))
    (:then_1
      (Utilities|Array|Add _playercontrollers NewPlayer))))

(event EventOnSwapPlayerControllers
  (params (OldPC :type Player%20Controller%20Object%20Reference) (NewPC :type Player%20Controller%20Object%20Reference))
  ;[0 0 0] Manage Connections
  ;;[1 1 1] On Player Login
  (Utilities|Array|Add (Variables|Default|GetPlayerControllers) NewPC))

(event EventOnLogout
  (params (ExitingController :type Controller%20Object%20Reference))
  ;[0 0 0] Manage Connections
  ;;[1 1 1] On Player Logout
  (bind _asbp_game_pc (Utilities|Casting|CastToBP_Game_PC ExitingController))
  (Utilities|Array|RemoveItem (Variables|Default|GetPlayerControllers) _asbp_game_pc))

(fn ConstructionScript)

(fn SpawnPlayer
  (params (Player%20Controller :type BP%20Game%20PC%20Object%20Reference))
  (bind _returnvalue (Pawn|GetControlledPawn Player%20Controller))
  (bind _transform (Spawning|FindRandomPlayerStart))
  ;[0 0.04485 0.4497] Delete Existing Pawn
  (Utilities|IsValid _returnvalue
    (:Is%20Valid
      (Actor|DestroyActor _returnvalue))
    (:Is%20Not%20Valid
      _))
  ;[1 1 1] Select Pawn
  (if (Variables|/Game/Blueprints/BP_Game_PC.BP_Game_PC_C|GetIsVR Player%20Controller)
    ;[0.1684 0.001512 0] Spawn VR Pawn
    (bind _returnvalue_2 (Game|SpawnActorfromClass "/Game/VRTemplate/Blueprints/VRPawn.VRPawn_C" _transform "Undefined" "MultiplyWithRoot" 0 0))
    (Pawn|Possess Player%20Controller _returnvalue_2)
    (Class|PrimitiveComponent|SetOwnerNoSee (Variables|/Game/VRTemplate/Blueprints/VRPawn.VRPawn_C|GetHandRight _returnvalue_2) false)
    (else
      ;[0 0.2448 0.01525] Spawn Ghost Pawn
      (bind _returnvalue_3 (Game|SpawnActorfromClass "/Game/ThirdPerson/Blueprints/BP_ThirdPersonCharacter.BP_ThirdPersonCharacter_C" _transform "Undefined" "MultiplyWithRoot" 0 0))
      (Pawn|Possess Player%20Controller _returnvalue_3)
      (Development|PrintString "Spawned Ghost"))))

(fn FindRandomPlayerStart
  (bind _playerspawns (Variables|Default|GetPlayerSpawns))
  (return (Transformation|GetActorTransform (Utilities|Array|Get(acopy) _playerspawns (Math|Random|RandomIntegerinRange 0 (- (Utilities|Array|Length _playerspawns) 1))))))

(fn GetPlayersinCaptureArea
  (params (Capture%20Area :type BP%20Capture%20Area%20Object%20Reference))
  (bind _playercount (LocalVariables|GetPlayerCount))
  (for _array_element (Variables|Default|GetPlayerControllers)
    (if (< (Math|Vector|Distance(Vector) (Transformation|GetActorLocation Capture%20Area) (Transformation|GetActorLocation (Pawn|GetControlledPawn _array_element))) (Variables|/Game/Blueprints/BP_CaptureArea.BP_CaptureArea_C|GetRadius Capture%20Area))
      (Math|Integer|IncrementInt _playercount)))
  (return _playercount))

(fn UpdateCaptureAreaStatus
  (for (_array_element _array_index) (Variables|Default|GetCaptureAreas)
    (bind _count (Ghosts|GetPlayersinCaptureArea _array_element))
    (Development|PrintString (Utilities|String|Append "Players around  " (Utilities|String|ToString(Integer) _array_index) ": " (Utilities|String|ToString(Integer) _count)))))

(fn UpdateVRDummy
  (params (Flashlight%20Transform :type Transform))
  (Transformation|SetActorTransform (Variables|Default|GetFlashlight) Flashlight%20Transform))